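; BP_DeskktopCaptureManager is an actor that captures the screen and shows the live image on its plane and in an on-screen widget.
; On BeginPlay it creates the widget and a dynamic MI_SimpleTexture material, then initializes capture and binds the resulting texture to both.
; A looping timer, rather than Tick, polls CaptureScreenSync and synchronously updates the shared texture when capture succeeds.
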(event `Sync tex update`
  ;[1 1 1] draw loop
  (bind _returnvalue (`self.CaptureScreenSync`))
  (if _returnvalue
    (`self.UpdateTextureSync`)))

(event `self.ReceiveBeginPlay`
  (bind _texture (`self.Texture`))
  ;[1 1 1] begin play
  (`|ExecutionSequence`
    (:`then_0`
      ;[1 1 1] spawn widget
      (bind _returnvalue (`|CreateWidget` "/Game/GeomOutput/NewWidgetBlueprint.NewWidgetBlueprint_C" (`GameplayStatics.GetPlayerController` 0)))
      (set `self.UI_Image` (`/Game/GeomOutput/NewWidgetBlueprint.Image_184` _returnvalue))
      (`UserWidget.AddToViewport` _returnvalue 0))
    (:`then_1`
      ;[1 1 1] create dynamic MI, assign to plane, set texture
      (bind _returnvalue_2 (`KismetMaterialLibrary.CreateDynamicMaterialInstance` "/Game/GeomOutput/MI_SimpleTexture.MI_SimpleTexture"))
      (bind _output_get (set `self.DMI` _returnvalue_2))
      (`PrimitiveComponent.SetMaterial` (`self.Plane`) 0 _output_get)
      (bind _returnvalue_3 (`self.InitCapture` 1))
      (if _returnvalue_3
        (bind _returnvalue_4 (`self.GetTexture`))
        (bind _output_get_2 (set `self.Texture` _returnvalue_4))
        (`MaterialInstanceDynamic.SetTextureParameterValue` (`self.DMI`) "Texture" _output_get_2)
        (bind _output_get_3 (set `self.Brush` (`WidgetBlueprintLibrary.MakeBrushFromTexture` _texture (`Texture2D.Blueprint_GetSizeX` _texture) (`Texture2D.Blueprint_GetSizeY` _texture))))
        (`Image.SetBrush` (`self.UI_Image`) _output_get_3)
        ;[1 1 1] draw loop
        (`KismetSystemLibrary.K2_SetTimerDelegate` (delegate `Sync tex update`) 0.05 true)
        (else
          (`KismetSystemLibrary.PrintString` "Hello"))))))

(fn `UserConstructionScript`)